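; BP_CroudPath is a crowd path actor that lays out NPC points along its Path spline at BeginPlay.
; PlaceNPCPoints sets existing points' lifespan to zero, which does not destroy them in Unreal, and clears the NPCPoints array.
; It then loops along the spline at fixed distance steps, spawning an NPC_Point at each world location and storing it in NPCPoints until the spline length is reached.
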(event `self.ReceiveBeginPlay`
  (`self.Place NPC Points`))

(event `Place NPC Points`
  ;[1 1 1] Initialisation du chemin (supprimé les points déja existant)
  (set `self.Distance` 0.0)
  (for _array_element (`self.NPC_Points`)
    (`self.SetLifeSpan` _array_element 0.0))
  (`KismetArrayLibrary.Array_Clear` (`self.NPC_Points`))
  ;[1 1 1] Spawn les points sur le chemin avec une distance de 400 entre chaque point
  (bind _returnvalue (`|SpawnActorFromClass` "/Game/SEFAR/Core/BluePrints/Croud/NPC_Point.NPC_Point_C" (`KismetMathLibrary.MakeTransform` (`SplineComponent.GetLocationAtDistanceAlongSpline` (`self.Path`) (`self.Distance`) "World")) "Undefined" "OverrideRootScale" null null :!label _label))
  ;[1 1 1] Créer un tableau des points
  (`KismetArrayLibrary.Array_Add` (`self.NPC_Points`) _returnvalue)
  ;[1 1 1] Vérifier si on a atteint la fin du chemin sinon spawn un autre point
  (bind _output_get (set `self.Distance` (+ (`self.Distance`) 400.0)))
  (if (< _output_get (`SplineComponent.GetSplineLength` (`self.Path`)))
    (goto _label)))

(fn `UserConstructionScript`)