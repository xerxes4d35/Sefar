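; AI controller for crowd pawns that wander endlessly between nearby point objects.
; NextPoint sphere-traces ahead of the pawn, widening the radius until it finds hits, and ignores the last stored actor.
; It moves to a reachable spot near a random hit, then searches again on success or after a short delay on failure.
; The stored actor and destination come from separate random picks, so they can differ.
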(event `self.ReceiveBeginPlay`
  (`KismetSystemLibrary.Delay` 0.1)
  (`self.Next_Point`))

(event `Go_to`
  (params (Target :type "Vector Structure"))
  ;[1 1 1] Bouger l'IA au prochain point
  (`|AIMoveTo` null Target null 100.0
    (:`OnSuccess`
      _)
    (:`OnFail`
      (`KismetSystemLibrary.Delay` 0.1)))
  (`self.Next_Point`))

(event `Next_Point`
  (bind _returnvalue (`self.K2_GetPawn`))
  (bind _returnvalue_2 (+ (`self.K2_GetActorLocation` _returnvalue) (* (`self.GetActorForwardVector` _returnvalue) (700.0 700.0 700.0))))
  ;[1 1 1] Calcule du prochain point
  (set `self.Radius` 600.0)
  (bind (_outhits _returnvalue_3) (`KismetSystemLibrary.SphereTraceMultiForObjects` _returnvalue_2 (+ _returnvalue_2 (1.0 0.0 0.0)) (`self.Radius`) (`|MakeArray` "ObjectTypeQuery8" :!type "EObjectTypeQuery Enum") false (`|MakeArray` (`self.Hit Actor`)) :!label _label))
  (if _returnvalue_3
    (bind (_bblockinghit _binitialoverlap _time _distance _location _impactpoint _normal _impactnormal _physmat _hitactor) (`GameplayStatics.BreakHitResult` (`|GetArrayItem` _outhits (`KismetMathLibrary.RandomInteger` (`KismetArrayLibrary.Array_Length` _outhits)))))
    (set `self.Hit Actor` _hitactor)
    (`self.Go_to` (`NavigationSystemV1.K2_GetRandomReachablePointInRadius` _impactpoint 100.0 null null))
    (else
      (set `self.Radius` (+ (`self.Radius`) 500.0))
      (`KismetSystemLibrary.Delay` 0.1)
      (goto _label))))

(fn `UserConstructionScript`)