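; BP_NPC_Interact is an NPC blueprint that opens a dialogue UI for interaction.
; ShowDialogue calls DisableInput, creates a BP_Dialogue_Widget with itself passed as the NPC, stores the reference and adds it to the viewport.
; The event graph holds only disabled default events, so nothing in this blueprint calls ShowDialogue itself.
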(fn `ShowDialogue`
  (`self.DisableInput` null)
  (bind _returnvalue (`|CreateWidget` "/Game/SEFAR/Core/BluePrints/BP_Dialogue_Widget.BP_Dialogue_Widget_C" null self))
  (bind _output_get (set `self.DialogueWidget` _returnvalue))
  (`UserWidget.AddToViewport` _output_get 0))

(fn `UserConstructionScript`
  (`parent.UserConstructionScript`))