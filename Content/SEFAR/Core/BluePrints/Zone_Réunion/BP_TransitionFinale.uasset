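; Trigger actor that stages the final standoff in the meeting zone and transitions to the ending level.
; On hero overlap it takes the camera, AI-moves the hero, Alsan and Durruti, sets aiming poses around Celia, plays dialogue, then restores control and shows the Astera03 widget.
; AsteraDone reads the GameInstance choice to play Alsan's or Celia's death with gunshots, then fades and opens LvL14END.
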(event `AsteraDone`
  (`KismetSystemLibrary.Delay` 0.5)
  (bind _asbp_game_instance (cast `/Game/SEFAR/Core/BluePrints/BP_GameInstance` (`GameplayStatics.GetGameInstance`)))
  (if (== (`/Game/SEFAR/Core/BluePrints/BP_GameInstance.Astera03_Choix` _asbp_game_instance) 2)
    (bind _returnvalue (`GameplayStatics.GetActorOfClass` "/Game/SEFAR/Core/BluePrints/BP_Durruti.BP_Durruti_C"))
    (`self.K2_AddActorLocalRotation` _returnvalue (struct :`Yaw` 90.0) false false)
    (`GameplayStatics.SpawnSoundAtLocation` "/Game/SEFAR/Sound/VFX/SD_Zone_Finale/Pistol_Shots.Pistol_Shots" (`self.LocationSound`) (struct) 1.0 1.0 0.0 null null)
    (`KismetSystemLibrary.Delay` 1.4)
    (bind _asbp_policier_animation (cast `/Game/SEFAR/Characters/PNJs/Policier/Animation/BP_PolicierAnimation` (`self.AlsanAnime`)))
    (set `/Game/SEFAR/Characters/PNJs/Policier/Animation/BP_PolicierAnimation.IsDead` true _asbp_policier_animation)
    (`KismetSystemLibrary.Delay` 3.45)
    (bind _returnvalue_2 (`|CreateWidget` "/Game/SEFAR/Core/BluePrints/Widget/Loading_Screen/LoadingScreenCinematicFadeIn.LoadingScreenCinematicFadeIn_C"))
    (`UserWidget.AddToViewport` _returnvalue_2 0)
    (`KismetSystemLibrary.Delay` 1.0)
    (bind _asbp_game_instance_2 (cast `/Game/SEFAR/Core/BluePrints/BP_GameInstance` (`GameplayStatics.GetGameInstance`)))
    (set `/Game/SEFAR/Core/BluePrints/BP_GameInstance.Level` 14 _asbp_game_instance_2)
    (`GameplayStatics.OpenLevel` "LvL14END")
    (else
      (`GameplayStatics.SpawnSoundAtLocation` "/Game/SEFAR/Sound/VFX/SD_Zone_Finale/Pistol_Shots.Pistol_Shots" (`self.LocationSound`) (struct) 1.0 1.0 0.0 null null)
      (`KismetSystemLibrary.Delay` 1.4)
      (bind _ascelia_anim_bp (cast `/Game/SEFAR/Characters/Celia/Animations/Celia_AnimBP` (`self.AnimeCelia`)))
      (set `/Game/SEFAR/Characters/Celia/Animations/Celia_AnimBP.IsDead` true _ascelia_anim_bp)
      (`KismetSystemLibrary.Delay` 2.45)
      (bind _returnvalue_3 (`|CreateWidget` "/Game/SEFAR/Core/BluePrints/Widget/Loading_Screen/LoadingScreenCinematicFadeIn.LoadingScreenCinematicFadeIn_C"))
      (`UserWidget.AddToViewport` _returnvalue_3 0)
      (`KismetSystemLibrary.Delay` 1.0)
      (bind _asbp_game_instance_3 (cast `/Game/SEFAR/Core/BluePrints/BP_GameInstance` (`GameplayStatics.GetGameInstance`)))
      (set `/Game/SEFAR/Core/BluePrints/BP_GameInstance.Level` 14 _asbp_game_instance_3)
      (`GameplayStatics.OpenLevel` "LvL14END"))))

(event `self.ReceiveActorBeginOverlap`
  (params (OtherActor :type "Actor Object Reference"))
  (bind _controller (`self.Controller`))
  (bind _asbp_hero (cast `/Game/SEFAR/Core/BluePrints/BP_Hero` OtherActor))
  (set `self.BP Hero` _asbp_hero)
  (bind _asbp_game_instance (cast `/Game/SEFAR/Core/BluePrints/BP_GameInstance` (`GameplayStatics.GetGameInstance`)))
  (if (`/Game/SEFAR/Core/BluePrints/BP_GameInstance.Subtitles` _asbp_game_instance)
    (`GameplayStatics.SetSubtitlesEnabled` true)
    (else
      (`GameplayStatics.SetSubtitlesEnabled` false)))
  (bind _output_get (set `self.Controller` (`GameplayStatics.GetPlayerController` 0)))
  (`PlayerController.SetViewTargetWithBlend` (`self.Controller`) self 1.0 "VTBlend_Linear" 0.0 false)
  (`Controller.UnPossess` _output_get)
  (`Pawn.SpawnDefaultController` (`self.BP Hero`))
  (`|AIMoveTo` (`self.BP Hero`) (`NavigationSystemV1.K2_GetRandomLocationInNavigableRadius` (`SceneComponent.K2_GetComponentLocation` (`self.Destination`)) 50.0 null null) null
    (:`OnSuccess`
      (bind _returnvalue (`GameplayStatics.GetActorOfClass` "/Game/SEFAR/Core/BluePrints/BP_Alsan.BP_Alsan_C"))
      (`|AIMoveTo` _returnvalue (`self.AlsanMoveLocation`) null
        (:`then`
          (set `self.AlsanAnime` (`SkeletalMeshComponent.GetAnimInstance` (`Character.Mesh` _returnvalue)))
          (bind _returnvalue_2 (`GameplayStatics.GetActorOfClass` "/Game/SEFAR/Core/BluePrints/BP_Durruti.BP_Durruti_C"))
          (`|AIMoveTo` _returnvalue_2 (`self.DurrutiMoveLocation`) null
            (:`OnSuccess`
              (set `self.AnimeDurruti` (`SkeletalMeshComponent.GetAnimInstance` (`Character.Mesh` _returnvalue_2)))
              (bind _returnvalue_3 (`GameplayStatics.GetActorOfClass` "/Game/SEFAR/Characters/Celia/BP_Celia.BP_Celia_C"))
              (set `self.AnimeCelia` (`SkeletalMeshComponent.GetAnimInstance` (`Character.Mesh` _returnvalue_3)))
              (bind _asbp_policier_animation (cast `/Game/SEFAR/Characters/PNJs/Policier/Animation/BP_PolicierAnimation` (`self.AlsanAnime`)))
              (set `/Game/SEFAR/Characters/PNJs/Policier/Animation/BP_PolicierAnimation.IsAiming` true _asbp_policier_animation)
              (bind _asbp_policier_animation_2 (cast `/Game/SEFAR/Characters/PNJs/Policier/Animation/BP_PolicierAnimation` (`self.AnimeDurruti`)))
              (set `/Game/SEFAR/Characters/PNJs/Policier/Animation/BP_PolicierAnimation.IsAiming` true _asbp_policier_animation_2)
              (bind _ascelia_anim_bp (cast `/Game/SEFAR/Characters/Celia/Animations/Celia_AnimBP` (`self.AnimeCelia`)))
              (set `/Game/SEFAR/Characters/Celia/Animations/Celia_AnimBP.IsAimed` true _ascelia_anim_bp)
              (`GameplayStatics.SpawnSoundAtLocation` "/Game/SEFAR/Sound/Dialogue/Zone_Finale/Scene26.Scene26" (`self.LocationSound`) (struct) 1.0 1.0 0.0 null null)
              (`KismetSystemLibrary.Delay` 10.53)
              (`Controller.UnPossess` (`Pawn.GetController` (`self.BP Hero`)))
              (`Controller.Possess` _controller (`self.BP Hero`))
              (`PlayerController.SetViewTargetWithBlend` _controller (`self.BP Hero`) 1.0 "VTBlend_Linear" 0.0 false)
              (`/Game/SEFAR/Core/BluePrints/BP_Hero.DisplayWBPAstera03` (`self.BP Hero`) true))))))))

(fn `UserConstructionScript`)