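; BP_DURRUTI is an actor that spawns a BP_ALSAN actor at a hardcoded transform when its PlayDialogue flag is false.
; Tick polls the flag, and a DoOnce limits the spawn to the first frame the flag reads false, ignoring collisions.
; Nothing in this Blueprint sets PlayDialogue, and the construction script only calls its parent.
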(event `self.ReceiveTick`
  (params (DeltaSeconds :type "Float (single-precision)"))
  (if (not (`self.PlayDialogue`))
    (`/Engine/EditorBlueprintResources/StandardMacros.DoOnce` false
      (:`Completed`
        (`|SpawnActorFromClass` :`Class` "/Game/SEFAR/Core/BluePrints/BP_ALSAN.BP_ALSAN_C" :`SpawnTransform` (`KismetMathLibrary.MakeTransform` (212.0 -210.0 194.0)) :`CollisionHandlingOverride` "AlwaysSpawn" :`TransformScaleMethod` "OverrideRootScale" :`Instigator` null)))))

(fn `UserConstructionScript`
  (`parent.UserConstructionScript`))