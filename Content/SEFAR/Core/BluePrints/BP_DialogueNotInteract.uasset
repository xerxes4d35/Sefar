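; Trigger actor that displays non-interactive dialogue when something overlaps its Box.
; The first overlap passes a DoOnce and, if PlayDialogue is set, creates WBP_DialogueNotInteract_Widget with a reference to this actor and adds it to the viewport.
; A separate hide function, not called within this Blueprint, clears PlayDialogue and removes the widget.
; The overlap does not filter which actor triggers it.
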(event `self.Box.OnComponentBeginOverlap`
  (params (OverlappedComponent :type "PrimitiveComponent Object Reference") (OtherActor :type "Actor Object Reference") (OtherComp :type "PrimitiveComponent Object Reference") (OtherBodyIndex :type Integer) (bFromSweep :type Boolean) (SweepResult :type "HitResult Structure (by ref)"))
  (`/Engine/EditorBlueprintResources/StandardMacros.DoOnce` false
    (:`Completed`
      (`self.Not Interact Show Dialogue`))))

(fn `Not Interact Show Dialogue`
  (if (`self.PlayDialogue`)
    (bind _returnvalue (`|CreateWidget` "/Game/SEFAR/Core/BluePrints/Widget/Dialogue/WBP_DialogueNotInteract_Widget.WBP_DialogueNotInteract_Widget_C" null self))
    (bind _output_get (set `self.WBPDialogueNotInteract` _returnvalue))
    (`UserWidget.AddToViewport` _output_get 0)))

(fn `NotInteract_HideDialogue`
  (set `self.PlayDialogue` false)
  (`Widget.RemoveFromParent` (`self.WBPDialogueNotInteract`)))

(fn `UserConstructionScript`)