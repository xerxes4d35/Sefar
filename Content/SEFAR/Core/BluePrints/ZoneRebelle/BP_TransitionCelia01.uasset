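; BP_TransitionCelia01 is a one-shot trigger in ZoneRebelle that plays a scripted, audio-driven transition scene when BP_Hero enters it.
; It blends the camera to itself and swaps the hero to an AI controller to walk near a destination point.
; On arrival it plays Scene_17, then a follow-up chosen by the GameInstance's Astera01Choix, timed with hardcoded delays.
; It then restores player possession and the hero camera.
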(event `self.ReceiveActorBeginOverlap`
  (params (OtherActor :type "Actor Object Reference"))
  (bind _controller (`self.Controller`))
  (bind _bp_hero (`self.BP Hero`))
  (bind _asbp_hero (cast `/Game/SEFAR/Core/BluePrints/BP_Hero` OtherActor))
  (set `self.BP Hero` _asbp_hero)
  (bind _asbp_game_instance (cast `/Game/SEFAR/Core/BluePrints/BP_GameInstance` (`GameplayStatics.GetGameInstance`)))
  (`GameplayStatics.SetSubtitlesEnabled` (`/Game/SEFAR/Core/BluePrints/BP_GameInstance.Subtitles` _asbp_game_instance))
  (if (not (`self.GetOverlapped`))
    (set `self.Controller` (`GameplayStatics.GetPlayerController` 0))
    (`PlayerController.SetViewTargetWithBlend` (`self.Controller`) self 1.0 "VTBlend_Linear" 0.0 false)
    (set `self.GetOverlapped` true)
    (`Controller.UnPossess` (`self.Controller`))
    (`Pawn.SpawnDefaultController` _bp_hero)
    (`|AIMoveTo` _bp_hero (`NavigationSystemV1.K2_GetRandomLocationInNavigableRadius` (`SceneComponent.K2_GetComponentLocation` (`self.Destination`)) 50.0 null null) null
      (:`OnSuccess`
        (`GameplayStatics.PlaySound2D` "/Game/SEFAR/Sound/Dialogue/Zone_Rebelle/Scene_17.Scene_17" 1.0 1.0 0.0 null null)
        (`KismetSystemLibrary.Delay` 55.0)
        (bind _asbp_game_instance_2 (cast `/Game/SEFAR/Core/BluePrints/BP_GameInstance` (`GameplayStatics.GetGameInstance`)))
        ;[1 1 1] 0 = Joie (Adam arrêté)
        ; 1 = Tristesse (Adam arrêté)
        ; 2 = Colère (Adam vient)
        ; 3 = Peur (Adam sort boutique)
        (switch `int` (`/Game/SEFAR/Core/BluePrints/BP_GameInstance.Astera01_Choix` _asbp_game_instance_2) ; Default: only to test here
          (:`Default`
            (`GameplayStatics.PlaySound2D` "/Game/SEFAR/Sound/Dialogue/Zone_Rebelle/Scene_17_1.Scene_17_1" 1.0 1.0 0.0 null null :!label _label) ; Adam vient
            (`KismetSystemLibrary.Delay` 16.0))
          (:`0`
            (`GameplayStatics.PlaySound2D` "/Game/SEFAR/Sound/Dialogue/Zone_Rebelle/Scene_17_3.Scene_17_3" 1.0 1.0 0.0 null null :!label _label_2)
            (`KismetSystemLibrary.Delay` 24.5))
          (:`1`
            (goto _label_2))
          (:`2`
            (goto _label))
          (:`3`
            (`GameplayStatics.PlaySound2D` "/Game/SEFAR/Sound/Dialogue/Zone_Rebelle/Scene_17_2.Scene_17_2" 1.0 1.0 0.0 null null)
            (`KismetSystemLibrary.Delay` 22.18)))
        (`Controller.UnPossess` (`Pawn.GetController` (`self.BP Hero`)))
        (`Controller.Possess` _controller (`self.BP Hero`))
        (`PlayerController.SetViewTargetWithBlend` _controller (`self.BP Hero`) 1.0 "VTBlend_Linear" 0.0 false)))))

(fn `UserConstructionScript`)