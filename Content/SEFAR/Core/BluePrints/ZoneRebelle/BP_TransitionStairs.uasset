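; BP_TransitionStairs is a trigger actor that automatically walks BP_Hero through a stairs transition in ZoneRebelle.
; On hero overlap, it runs only if BP_TransitionLouiza reports it was overlapped, then blends the view to itself.
; It swaps the player controller for a default AI controller to move the hero near the Destination component.
; After a successful move and short delay, it restores player possession and the hero camera, with no failure branch.
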(event `self.ReceiveActorBeginOverlap`
  (params (OtherActor :type "Actor Object Reference"))
  (bind _controller (`self.Controller`))
  (bind _bp_hero (`self.BP Hero`))
  (bind _asbp_hero (cast `/Game/SEFAR/Core/BluePrints/BP_Hero` OtherActor))
  (set `self.BP Hero` _asbp_hero)
  (set `self.Controller` (`GameplayStatics.GetPlayerController` 0))
  (bind _returnvalue (`GameplayStatics.GetActorOfClass` "/Game/SEFAR/Core/BluePrints/ZoneRebelle/BP_TransitionLouiza.BP_TransitionLouiza_C"))
  (if (`/Game/SEFAR/Core/BluePrints/ZoneRebelle/BP_TransitionLouiza.GetOverlapped` _returnvalue)
    (set `self.Transition_Camera` (`/Game/SEFAR/Core/BluePrints/BP_Hero.Camera` (`self.BP Hero`)))
    (`PlayerController.SetViewTargetWithBlend` (`self.Controller`) self 0.2 "VTBlend_Linear" 0.0 false)
    (`Controller.UnPossess` (`self.Controller`))
    (`Pawn.SpawnDefaultController` _bp_hero)
    (`|AIMoveTo` _bp_hero (`NavigationSystemV1.K2_GetRandomLocationInNavigableRadius` (`SceneComponent.K2_GetComponentLocation` (`self.Destination`)) 50.0 null null) null
      (:`OnSuccess`
        (`KismetSystemLibrary.Delay` 1.0)
        (`Controller.UnPossess` (`Pawn.GetController` (`self.BP Hero`)))
        (`Controller.Possess` _controller (`self.BP Hero`))
        (`PlayerController.SetViewTargetWithBlend` _controller (`self.BP Hero`) 0.3 "VTBlend_Linear" 0.0 false)))))

(fn `UserConstructionScript`)