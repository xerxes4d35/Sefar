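; Rebel-zone journal interactable that lets the hero open Melinda's report on screen.
; Overlapping AsteraTrigger shows the A-button prompt once BP_TransitionJugo's dialogue is done and until the report interaction is completed.
; A shows the report if the GameInstance's TriggerAsteraJugo flag is set, otherwise plays a voice scene sound.
; B hides the report, displays an Astera widget on the hero and disables further overlap prompts.
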(event `BouttonBPressed`
  (`Widget.SetVisibility` (`/Game/SEFAR/Core/BluePrints/BP_Hero.Rapport_Melinda` (`self.BP Hero`)) "Collapsed")
  ;[1 1 1] Juste ça ?
  (`/Game/SEFAR/Core/BluePrints/BP_Hero.DisplayWBPAstera02` (`self.BP Hero`) true)
  (set `self.GetOverlaped` true))

(event `BouttonAPressed`
  (bind _asbp_hero (cast `/Game/SEFAR/Core/BluePrints/BP_Hero` (`GameplayStatics.GetPlayerPawn` 0)))
  (set `self.BP Hero` _asbp_hero)
  (bind _asbp_game_instance (cast `/Game/SEFAR/Core/BluePrints/BP_GameInstance` (`GameplayStatics.GetGameInstance`)))
  (if (`/Game/SEFAR/Core/BluePrints/BP_GameInstance.TriggerAsteraJugo` _asbp_game_instance)
    (`Widget.SetVisibility` (`/Game/SEFAR/Core/BluePrints/BP_Hero.Rapport_Melinda` (`self.BP Hero`)) "Visible")
    (set `self.IsRapportVisible` true)
    (else
      (`GameplayStatics.PlaySound2D` "/Game/SEFAR/Sound/Dialogue/Zone_Rebelle/Scene_19_BIS.Scene_19_BIS" 1.0 1.0 0.0 null null))))

(event `self.AsteraTrigger.OnComponentBeginOverlap`
  (params (OverlappedComponent :type "PrimitiveComponent Object Reference") (OtherActor :type "Actor Object Reference") (OtherComp :type "PrimitiveComponent Object Reference") (OtherBodyIndex :type Integer) (bFromSweep :type Boolean) (SweepResult :type "HitResult Structure (by ref)"))
  (bind _returnvalue (`GameplayStatics.GetActorOfClass` "/Game/SEFAR/Core/BluePrints/ZoneRebelle/BP_TransitionJugo.BP_TransitionJugo_C"))
  (if (`/Game/SEFAR/Core/BluePrints/ZoneRebelle/BP_TransitionJugo.IsDialogueDone` _returnvalue)
    (bind _asbp_hero (cast `/Game/SEFAR/Core/BluePrints/BP_Hero` OtherActor))
    (bind _output_get (set `self.BP Hero` _asbp_hero))
    (if (not (`self.GetOverlaped`))
      (`Widget.SetVisibility` (`/Game/SEFAR/Core/BluePrints/BP_Hero.BouttonA` _output_get) "Visible")
      (set `self.IsBouttonAVisible` true))))

(event `self.AsteraTrigger.OnComponentEndOverlap`
  (params (OverlappedComponent :type "PrimitiveComponent Object Reference") (OtherActor :type "Actor Object Reference") (OtherComp :type "PrimitiveComponent Object Reference") (OtherBodyIndex :type Integer))
  (bind _asbp_hero (cast `/Game/SEFAR/Core/BluePrints/BP_Hero` OtherActor))
  (if (not (`self.GetOverlaped`))
    (`Widget.SetVisibility` (`/Game/SEFAR/Core/BluePrints/BP_Hero.BouttonA` _asbp_hero) "Collapsed")
    (set `self.IsBouttonAVisible` false)))

(fn `UserConstructionScript`)