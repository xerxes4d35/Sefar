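; BP_TransitionLouiza is an overlap-triggered cinematic transition for the scene with Louiza.
; On hero overlap it applies the subtitle setting and, until completed once, blends the view to itself and hands the hero to AI.
; The hero walks to a mark, Scene_20 audio plays through a fixed delay, then Louiza starts walking off.
; Meanwhile Arrawis01 and Jugo are destroyed, TriggerAsteraJugo is set, and the hero walks to a final point where player control returns.
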(event `self.ReceiveActorBeginOverlap`
  (params (OtherActor :type "Actor Object Reference"))
  (bind _bp_hero (`self.BP Hero`))
  (bind _controller (`self.Controller`))
  (bind _asbp_hero (cast `/Game/SEFAR/Core/BluePrints/BP_Hero` OtherActor))
  (set `self.BP Hero` _asbp_hero)
  (bind _asbp_game_instance (cast `/Game/SEFAR/Core/BluePrints/BP_GameInstance` (`GameplayStatics.GetGameInstance`)))
  (if (`/Game/SEFAR/Core/BluePrints/BP_GameInstance.Subtitles` _asbp_game_instance)
    (`GameplayStatics.SetSubtitlesEnabled` true)
    (else
      (`GameplayStatics.SetSubtitlesEnabled` false)))
  (set `self.Controller` (`GameplayStatics.GetPlayerController` 0))
  (if (not (`self.GetOverlapped`))
    (`PlayerController.SetViewTargetWithBlend` (`self.Controller`) self 1.0 "VTBlend_Linear" 0.0 false)
    (`Controller.UnPossess` (`self.Controller`))
    (`Pawn.SpawnDefaultController` _bp_hero)
    (`|AIMoveTo` _bp_hero (`NavigationSystemV1.K2_GetRandomLocationInNavigableRadius` (`SceneComponent.K2_GetComponentLocation` (`self.Destination`)) 50.0 null null) null
      (:`OnSuccess`
        (`GameplayStatics.PlaySound2D` "/Game/SEFAR/Sound/Dialogue/Zone_Rebelle/Scene_20.Scene_20" 1.0 1.0 0.0 null null)
        (`KismetSystemLibrary.Delay` 45.400002)
        (set `self.GetOverlapped` true)
        (bind _returnvalue (`GameplayStatics.GetActorOfClass` "/Game/SEFAR/Characters/Louiza/BP_Louiza.BP_Louiza_C"))
        (`|AIMoveTo` _returnvalue (`NavigationSystemV1.K2_GetRandomLocationInNavigableRadius` (`SceneComponent.K2_GetComponentLocation` (`self.DestroyLouiza`)) 50.0 null null) null
          (:`then`
            (bind _returnvalue_2 (`GameplayStatics.GetActorOfClass` "/Game/SEFAR/Characters/Arrawis01/BP_Arrawis01.BP_Arrawis01_C"))
            (`self.K2_DestroyActor` _returnvalue_2)
            (bind _returnvalue_3 (`GameplayStatics.GetActorOfClass` "/Game/SEFAR/Characters/Jugo/BP_Jugo.BP_Jugo_C"))
            (`self.K2_DestroyActor` _returnvalue_3)
            (bind _asbp_game_instance_2 (cast `/Game/SEFAR/Core/BluePrints/BP_GameInstance` (`GameplayStatics.GetGameInstance`)))
            (set `/Game/SEFAR/Core/BluePrints/BP_GameInstance.TriggerAsteraJugo` true _asbp_game_instance_2)
            (`|AIMoveTo` (`self.BP Hero`) (`NavigationSystemV1.K2_GetRandomLocationInNavigableRadius` (`SceneComponent.K2_GetComponentLocation` (`self.FinalDestination`)) 50.0 null null) null
              (:`OnSuccess`
                (`Controller.UnPossess` (`Pawn.GetController` (`self.BP Hero`)))
                (`Controller.Possess` _controller (`self.BP Hero`))
                (`PlayerController.SetViewTargetWithBlend` _controller (`self.BP Hero`) 1.0 "VTBlend_Linear" 0.0 false)))))))))

(fn `UserConstructionScript`)