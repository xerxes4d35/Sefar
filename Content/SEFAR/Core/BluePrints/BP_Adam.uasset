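; BP_Adam is an AI-moved character, Adam, that performs a scripted walk when the hero reaches him in level 4.
; A capsule overlap with BP_Hero checks the level stored in BP_GameInstance, with only level 4 handled.
; After a long fixed delay, AIMoveTo targets a random reachable point near Destination.
; On arrival, the mesh makes a quarter turn.
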(event `self.CapsuleComponent.OnComponentBeginOverlap`
  (params (OverlappedComponent :type "PrimitiveComponent Object Reference") (OtherActor :type "Actor Object Reference") (OtherComp :type "PrimitiveComponent Object Reference") (OtherBodyIndex :type Integer) (bFromSweep :type Boolean) (SweepResult :type "HitResult Structure (by ref)"))
  (cast `/Game/SEFAR/Core/BluePrints/BP_Hero` OtherActor)
  (bind _asbp_game_instance (cast `/Game/SEFAR/Core/BluePrints/BP_GameInstance` (`GameplayStatics.GetGameInstance`)))
  (switch `int` (`/Game/SEFAR/Core/BluePrints/BP_GameInstance.Level` _asbp_game_instance)
    (:`4`
      (`KismetSystemLibrary.Delay` 21.23)
      (`|AIMoveTo` (`self.GetController` self) null (`NavigationSystemV1.K2_GetRandomReachablePointInRadius` (`self.Destination`) 50.0 null null) null
        (:`OnSuccess`
          (`SceneComponent.K2_AddLocalRotation` (`self.Mesh`) (struct :`Yaw` -90.0) false false))))))

(fn `UserConstructionScript`)