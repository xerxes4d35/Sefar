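; Hidden door in Adam's shop (Magasin_Adam) that moves the player on to the Monologue_03 level.
; When BP_Hero enters its sphere, the game instance's Astera01Choix decides whether it opens: after Adam's talk, immediately, or once he is gone and the report is read.
; Most paths fade through a loading widget, but the report path shows the A-button prompt and loads immediately.
; A separate BouttonA event also triggers the faded transition.
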(event `BouttonA`
  (bind _returnvalue (`|CreateWidget` "/Game/SEFAR/Core/BluePrints/Widget/Loading_Screen/LoadingScreenCinematicFadeIn.LoadingScreenCinematicFadeIn_C"))
  (`UserWidget.AddToViewport` _returnvalue 0)
  (`KismetSystemLibrary.Delay` 1.0)
  (`GameplayStatics.OpenLevel` "Monologue_03"))

(event `self.Sphere.OnComponentBeginOverlap`
  (params (OverlappedComponent :type "PrimitiveComponent Object Reference") (OtherActor :type "Actor Object Reference") (OtherComp :type "PrimitiveComponent Object Reference") (OtherBodyIndex :type Integer) (bFromSweep :type Boolean) (SweepResult :type "HitResult Structure (by ref)"))
  (bind _asbp_hero (cast `/Game/SEFAR/Core/BluePrints/BP_Hero` OtherActor))
  (set `self.BP Hero` _asbp_hero)
  (bind _asbp_game_instance (cast `/Game/SEFAR/Core/BluePrints/BP_GameInstance` (`GameplayStatics.GetGameInstance`)))
  (switch `int` (`/Game/SEFAR/Core/BluePrints/BP_GameInstance.Astera01_Choix` _asbp_game_instance)
    (:`0`
      (bind _returnvalue (`GameplayStatics.GetActorOfClass` "/Game/SEFAR/Core/BluePrints/Magasin_Adam/BP_InteractionPainting.BP_InteractionPainting_C" :!label _label))
      (if (`/Game/SEFAR/Core/BluePrints/Magasin_Adam/BP_InteractionPainting.IsAdamEndTalk` _returnvalue)
        (bind _returnvalue_2 (`|CreateWidget` "/Game/SEFAR/Core/BluePrints/Widget/Loading_Screen/LoadingScreenCinematicFadeIn.LoadingScreenCinematicFadeIn_C"))
        (`UserWidget.AddToViewport` _returnvalue_2 0)
        (`KismetSystemLibrary.Delay` 1.0)
        (`GameplayStatics.OpenLevel` "Monologue_03")))
    (:`1`
      (goto _label))
    (:`2`
      (bind _returnvalue_3 (`|CreateWidget` "/Game/SEFAR/Core/BluePrints/Widget/Loading_Screen/LoadingScreenCinematicFadeIn.LoadingScreenCinematicFadeIn_C"))
      (`UserWidget.AddToViewport` _returnvalue_3 0)
      (`KismetSystemLibrary.Delay` 1.0)
      (`GameplayStatics.OpenLevel` "Monologue_03"))
    (:`3`
      (bind _returnvalue_4 (`GameplayStatics.GetActorOfClass` "/Game/SEFAR/Core/BluePrints/Magasin_Adam/BP_InteractionPainting.BP_InteractionPainting_C"))
      (if (`/Game/SEFAR/Core/BluePrints/Magasin_Adam/BP_InteractionPainting.IsAdamGone` _returnvalue_4)
        ;[1 0.1427 0.2124] Ne pas oublié de créer un bool dans gameinstance pour verifié qu'il a bien trouvé l'indice sur celia
        (bind _returnvalue_5 (`GameplayStatics.GetActorOfClass` "/Game/SEFAR/Core/BluePrints/Magasin_Adam/BP_DocumentInteract.BP_DocumentInteract_C"))
        (if (`/Game/SEFAR/Core/BluePrints/Magasin_Adam/BP_DocumentInteract.IsRapportReadden` _returnvalue_5)
          (`Widget.SetVisibility` (`/Game/SEFAR/Core/BluePrints/BP_Hero.BouttonA` (`self.BP Hero`)) "Visible")
          (`GameplayStatics.OpenLevel` "Monologue_03"))))))

(event `self.Sphere.OnComponentEndOverlap`
  (params (OverlappedComponent :type "PrimitiveComponent Object Reference") (OtherActor :type "Actor Object Reference") (OtherComp :type "PrimitiveComponent Object Reference") (OtherBodyIndex :type Integer))
  (bind _asbp_hero (cast `/Game/SEFAR/Core/BluePrints/BP_Hero` OtherActor))
  (set `self.BP Hero` _asbp_hero)
  (bind _asbp_game_instance (cast `/Game/SEFAR/Core/BluePrints/BP_GameInstance` (`GameplayStatics.GetGameInstance`)))
  (switch `int` (`/Game/SEFAR/Core/BluePrints/BP_GameInstance.Astera01_Choix` _asbp_game_instance)
    (:`3`
      (`Widget.SetVisibility` (`/Game/SEFAR/Core/BluePrints/BP_Hero.BouttonA` (`self.BP Hero`)) "Collapsed"))))

(fn `UserConstructionScript`)