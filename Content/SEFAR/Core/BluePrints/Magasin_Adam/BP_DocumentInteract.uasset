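; BP_DocumentInteract is an interactable document in Adam's shop (Magasin_Adam) that reveals Celia's report on the hero's UI.
; Box overlap shows the hero's A-button prompt only when Astera01Choix is 3, BP_InteractionPainting reports Adam gone and GetOverlapped is false.
; Leaving the box hides the prompt under the same GetOverlapped check.
; BouttonApressed and BouttonACollapse both make the report visible, without checking prompt visibility.
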(event `BouttonACollapse`
  (`Widget.SetVisibility` (`/Game/SEFAR/Core/BluePrints/BP_Hero.Rapport_Celia` (`self.BP Hero`)) "Visible"))

(event `BouttonApressed`
  (`Widget.SetVisibility` (`/Game/SEFAR/Core/BluePrints/BP_Hero.Rapport_Celia` (`self.BP Hero`)) "Visible"))

(event `self.Box.OnComponentBeginOverlap`
  (params (OverlappedComponent :type "PrimitiveComponent Object Reference") (OtherActor :type "Actor Object Reference") (OtherComp :type "PrimitiveComponent Object Reference") (OtherBodyIndex :type Integer) (bFromSweep :type Boolean) (SweepResult :type "HitResult Structure (by ref)"))
  (bind _asbp_hero (cast `/Game/SEFAR/Core/BluePrints/BP_Hero` OtherActor))
  (bind _output_get (set `self.BP Hero` _asbp_hero))
  (bind _asbp_game_instance (cast `/Game/SEFAR/Core/BluePrints/BP_GameInstance` (`GameplayStatics.GetGameInstance`)))
  (if (== (`/Game/SEFAR/Core/BluePrints/BP_GameInstance.Astera01_Choix` _asbp_game_instance) 3)
    (bind _returnvalue (`GameplayStatics.GetActorOfClass` "/Game/SEFAR/Core/BluePrints/Magasin_Adam/BP_InteractionPainting.BP_InteractionPainting_C"))
    (if (`/Game/SEFAR/Core/BluePrints/Magasin_Adam/BP_InteractionPainting.IsAdamGone` _returnvalue)
      (if (not (`self.GetOverlapped`))
        (`Widget.SetVisibility` (`/Game/SEFAR/Core/BluePrints/BP_Hero.BouttonA` _output_get) "Visible")
        (set `self.Is Boutton AVisible` true)))))

(event `self.Box.OnComponentEndOverlap`
  (params (OverlappedComponent :type "PrimitiveComponent Object Reference") (OtherActor :type "Actor Object Reference") (OtherComp :type "PrimitiveComponent Object Reference") (OtherBodyIndex :type Integer))
  (bind _asbp_hero (cast `/Game/SEFAR/Core/BluePrints/BP_Hero` OtherActor))
  (bind _output_get (set `self.BP Hero` _asbp_hero))
  (if (not (`self.GetOverlapped`))
    (`Widget.SetVisibility` (`/Game/SEFAR/Core/BluePrints/BP_Hero.BouttonA` _output_get) "Collapsed")
    (set `self.Is Boutton AVisible` false)))

(fn `UserConstructionScript`)