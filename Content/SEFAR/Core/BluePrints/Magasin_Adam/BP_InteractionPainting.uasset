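; Story interaction actor for a painting that plays a voiced cinematic scene and stages Adam's branching follow-up.
; A trigger shows the hero's A prompt; pressing it once blends the camera to this actor, AI-walks the hero into place, plays dialogue, then restores control.
; Astera_01_Choice reads the GameInstance choice to sequence sounds and Adam's movements with hard-coded delays, flagging his talk as ended or destroying him.
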(event `Astera_01_Choice`
  (bind _bp_adam (`self.BP_Adam`))
  (bind _asbp_game_instance (cast `/Game/SEFAR/Core/BluePrints/BP_GameInstance` (`GameplayStatics.GetGameInstance`)))
  (bind _returnvalue (`GameplayStatics.GetActorOfClass` "/Game/SEFAR/Core/BluePrints/BP_Hero.BP_Hero_C"))
  (set `self.BP_Hero02` _returnvalue)
  (if (`/Game/SEFAR/Core/BluePrints/BP_GameInstance.Subtitles` _asbp_game_instance)
    (`GameplayStatics.SetSubtitlesEnabled` true)
    (else
      (`GameplayStatics.SetSubtitlesEnabled` false)))
  (set `self.Controller_02` (`GameplayStatics.GetPlayerController` 0))
  (bind _outactors (`GameplayStatics.GetAllActorsOfClass` "/Game/SEFAR/Core/BluePrints/BP_Adam.BP_Adam_C"))
  (set `self.BP_Adam` (`|GetArrayItem` _outactors))
  (bind _asbp_game_instance_2 (cast `/Game/SEFAR/Core/BluePrints/BP_GameInstance` (`GameplayStatics.GetGameInstance`)))
  (switch `int` (`/Game/SEFAR/Core/BluePrints/BP_GameInstance.Astera01_Choix` _asbp_game_instance_2)
    (:`0`
      (`GameplayStatics.PlaySound2D` "/Game/SEFAR/Sound/VFX/SD_MagasinAdam/Phone_Ringing.Phone_Ringing" 1.0 1.0 0.0 null null)
      (`KismetSystemLibrary.Delay` 8.0)
      (bind _randomlocation (`NavigationSystemV1.K2_GetRandomLocationInNavigableRadius` (`self.Destination_Telephone`) 0.0 null null))
      (`|AIMoveTo` (`self.BP_Adam`) _randomlocation null
        (:`then`
          (`KismetSystemLibrary.Delay` 2.0)
          (`GameplayStatics.PlaySound2D` "/Game/SEFAR/Sound/Dialogue/Magasin_Adam/Scene14_3.Scene14_3" 1.0 1.0 0.0 null null)
          (`KismetSystemLibrary.Delay` 48.0)
          (bind _randomlocation_2 (`NavigationSystemV1.K2_GetRandomLocationInNavigableRadius` (`self.Destination_Adam_2`) 0.0 null null))
          (`|AIMoveTo` (`self.BP_Adam`) _randomlocation_2 null
            (:`then`
              (`KismetSystemLibrary.Delay` 16.5)
              (set `self.IsAdamEndTalk` true))))))
    (:`1`
      (`GameplayStatics.PlaySound2D` "/Game/SEFAR/Sound/VFX/SD_MagasinAdam/Phone_Ringing.Phone_Ringing" 1.0 1.0 0.0 null null)
      (`KismetSystemLibrary.Delay` 8.0)
      (bind _randomlocation_3 (`NavigationSystemV1.K2_GetRandomLocationInNavigableRadius` (`self.Destination_Telephone`) 0.0 null null))
      (`|AIMoveTo` (`self.BP_Adam`) _randomlocation_3 null
        (:`then`
          (`KismetSystemLibrary.Delay` 2.0)
          (`GameplayStatics.PlaySound2D` "/Game/SEFAR/Sound/Dialogue/Magasin_Adam/Scene14_2.Scene14_2" 1.0 1.0 0.0 null null)
          (`KismetSystemLibrary.Delay` 56.0)
          (bind _randomlocation_4 (`NavigationSystemV1.K2_GetRandomLocationInNavigableRadius` (`self.Destination_Adam_2`) 0.0 null null))
          (`|AIMoveTo` (`self.BP_Adam`) _randomlocation_4 null
            (:`then`
              (`KismetSystemLibrary.Delay` 12.8)
              (set `self.IsAdamEndTalk` true))))))
    (:`2`
      (`GameplayStatics.PlaySound2D` "/Game/SEFAR/Sound/Dialogue/Magasin_Adam/Scene14_4.Scene14_4" 1.0 1.0 0.0 null null)
      (`KismetSystemLibrary.Delay` 22.559999)
      (bind _randomlocation_5 (`NavigationSystemV1.K2_GetRandomLocationInNavigableRadius` (`self.Destination_Adam_2`) 0.0 null null))
      (`|AIMoveTo` (`self.BP_Adam`) _randomlocation_5 null))
    (:`3`
      (`GameplayStatics.PlaySound2D` "/Game/SEFAR/Sound/VFX/SD_MagasinAdam/Phone_Ringing.Phone_Ringing" 1.0 1.0 0.0 null null)
      (`KismetSystemLibrary.Delay` 8.0)
      (bind _randomlocation_6 (`NavigationSystemV1.K2_GetRandomLocationInNavigableRadius` (`self.Destination_Telephone`) 0.0 null null))
      (`|AIMoveTo` (`self.BP_Adam`) _randomlocation_6 null
        (:`then`
          (`KismetSystemLibrary.Delay` 2.0)
          (`GameplayStatics.PlaySound2D` "/Game/SEFAR/Sound/Dialogue/Magasin_Adam/Scene14_1.Scene14_1" 1.0 1.0 0.0 null null)
          (`KismetSystemLibrary.Delay` 23.5)
          (bind _randomlocation_7 (`NavigationSystemV1.K2_GetRandomLocationInNavigableRadius` (`self.Destination_Adam`) 0.0 null null))
          (`|AIMoveTo` _bp_adam _randomlocation_7 null
            (:`OnSuccess`
              (`self.K2_DestroyActor` _bp_adam)
              (set `self.IsAdamGone` true))))))))

(event `BouttonA_Pressed`
  (bind _bp_hero (`self.BP Hero`))
  (bind _controller (`self.Controller`))
  (bind _bp_hero_2 (`self.BP Hero`))
  (bind _asbp_game_instance (cast `/Game/SEFAR/Core/BluePrints/BP_GameInstance` (`GameplayStatics.GetGameInstance`)))
  (if (`/Game/SEFAR/Core/BluePrints/BP_GameInstance.Subtitles` _asbp_game_instance)
    (`GameplayStatics.SetSubtitlesEnabled` true)
    (else
      (`GameplayStatics.SetSubtitlesEnabled` false)))
  (if (not (`self.GetOverlapped`))
    (bind _output_get (set `self.Controller` (`GameplayStatics.GetPlayerController` 0)))
    (`PlayerController.SetViewTargetWithBlend` (`self.Controller`) self 1.0 "VTBlend_Linear" 0.0 false)
    (set `self.GetOverlapped` true)
    (`Controller.UnPossess` _output_get)
    (`Pawn.SpawnDefaultController` _bp_hero_2)
    (`Widget.SetVisibility` (`/Game/SEFAR/Core/BluePrints/BP_Hero.BouttonA` (`self.BP Hero`)) "Collapsed")
    (`|AIMoveTo` _bp_hero_2 (`NavigationSystemV1.K2_GetRandomLocationInNavigableRadius` (`SceneComponent.K2_GetComponentLocation` (`self.Destination`)) 10.0 null null) null
      (:`OnSuccess`
        (`GameplayStatics.PlaySound2D` "/Game/SEFAR/Sound/Dialogue/Magasin_Adam/Scene13.Scene13" 1.0 1.0 0.0 null null)
        (`KismetSystemLibrary.Delay` 33.790001)
        (`Controller.UnPossess` (`Pawn.GetController` (`self.BP Hero`)))
        (`Controller.Possess` _controller _bp_hero)
        (`PlayerController.SetViewTargetWithBlend` _controller _bp_hero 1.0 "VTBlend_Linear" 0.0 false)))))

(event `self.AsteraTrigger.OnComponentBeginOverlap`
  (params (OverlappedComponent :type "PrimitiveComponent Object Reference") (OtherActor :type "Actor Object Reference") (OtherComp :type "PrimitiveComponent Object Reference") (OtherBodyIndex :type Integer) (bFromSweep :type Boolean) (SweepResult :type "HitResult Structure (by ref)"))
  (bind _asbp_hero (cast `/Game/SEFAR/Core/BluePrints/BP_Hero` OtherActor))
  (bind _output_get (set `self.BP Hero` _asbp_hero))
  (if (not (`self.GetOverlapped`))
    (`Widget.SetVisibility` (`/Game/SEFAR/Core/BluePrints/BP_Hero.BouttonA` _output_get) "Visible")
    (set `self.IsBouttonAVisible` true)))

(event `self.AsteraTrigger.OnComponentEndOverlap`
  (params (OverlappedComponent :type "PrimitiveComponent Object Reference") (OtherActor :type "Actor Object Reference") (OtherComp :type "PrimitiveComponent Object Reference") (OtherBodyIndex :type Integer))
  (bind _asbp_hero (cast `/Game/SEFAR/Core/BluePrints/BP_Hero` OtherActor))
  (if (not (`self.GetOverlapped`))
    (`Widget.SetVisibility` (`/Game/SEFAR/Core/BluePrints/BP_Hero.BouttonA` _asbp_hero) "Collapsed")
    (set `self.IsBouttonAVisible` false)))

(fn `UserConstructionScript`)