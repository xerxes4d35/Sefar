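; Wall-clip Blueprint that clips walls between the camera and the player through a material parameter.
; A looping timer runs a multi-object line trace from the camera along its forward vector, as long as the camera-to-player distance.
; Hit actors are tracked in current and previous wall lists to toggle the "Clip" scalar on their static mesh materials.
; When the trace finds nothing, a resettable DoOnce unclips the current walls and clears both lists.
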(event `self.ReceiveBeginPlay`
  ;[1 1 1] CheckOverlap
  (`KismetSystemLibrary.K2_SetTimerDelegate` (`|CreateDelegate` :!event `CheckOverlap`) 0.2 true))

(event `CheckOverlap`
  (bind (_start_trace _end_trace) (`self.Compute Trace`))
  (bind (_outhits _returnvalue) (`KismetSystemLibrary.LineTraceMultiForObjects` _start_trace _end_trace (`|MakeArray` "ObjectTypeQuery7" :!type "EObjectTypeQuery Enum")))
  (if _returnvalue
    ;[1 1 1] Wall Clip if there is a wall between camera and the player
    (for _array_element _outhits
      (bind _output_get (set `self.CurrentWall` (`.HitActor` (`GameplayStatics.BreakHitResult` _array_element))))
      (if (not (`KismetArrayLibrary.Array_Contains` (`self.CurrentWalls`) _output_get))
        (`KismetArrayLibrary.Array_AddUnique` (`self.CurrentWalls`) (`self.CurrentWall`))
        (for _array_element_2 (`self.CurrentWalls`)
          (`self.WallClip` _array_element_2 true))
        (for _array_element_3 (`self.PreviousWalls`)
          (`self.WallClip` _array_element_3)
          (`KismetArrayLibrary.Array_RemoveItem` (`self.CurrentWalls`) _array_element_3))
        (else
          (set `self.PreviousWalls` (`self.CurrentWalls`)))))
    (`self.ResetOnTraceLost`)
    (else
      ;[1 1 1] Reset the wall clip
      (`/Engine/EditorBlueprintResources/StandardMacros.DoOnce` false :!label _label
        (:`Completed`
          (for _array_element_4 (`self.CurrentWalls`)
            (`self.WallClip` _array_element_4))
          (`KismetArrayLibrary.Array_Clear` (`self.CurrentWalls`))
          (`KismetArrayLibrary.Array_Clear` (`self.PreviousWalls`)))))))

(event `ResetOnTraceLost`
  ;[1 1 1] Reset the wall clip
  (goto _label :!via `Reset`))

(fn `Compute Trace`
  (returns (`Start Trace` :type "Vector Structure") (`End Trace` :type "Vector Structure"))
  (bind _returnvalue (`PlayerCameraManager.GetCameraLocation` (`GameplayStatics.GetPlayerCameraManager` 0)))
  (return _returnvalue (+ _returnvalue (* (`KismetMathLibrary.GetForwardVector` (`PlayerCameraManager.GetCameraRotation` (`GameplayStatics.GetPlayerCameraManager` 0))) (`KismetMathLibrary.Vector_Distance` (`PlayerCameraManager.GetCameraLocation` (`GameplayStatics.GetPlayerCameraManager` 0)) (`self.K2_GetActorLocation` (`GameplayStatics.GetPlayerCharacter` 0)))))))

(fn `UserConstructionScript`)

(fn `WallClip`
  (params (Wall :type "Actor Object Reference") (Clip :type Boolean))
  (`/Engine/EditorBlueprintResources/StandardMacros.IsValid` (`self.GetComponentByClass` (`local.Wall`) "/Script/Engine.StaticMeshComponent")
    (:`Is Valid`
      (`MeshComponent.SetScalarParameterValueOnMaterials` (`self.GetComponentByClass` (`local.Wall`) "/Script/Engine.StaticMeshComponent") "Clip" (`KismetMathLibrary.Conv_BoolToDouble` (`local.Clip`))))))