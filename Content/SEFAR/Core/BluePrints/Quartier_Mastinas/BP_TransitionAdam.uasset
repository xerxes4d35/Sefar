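; BP_TransitionAdam is a trigger actor in Quartier_Mastinas that takes control away from the player and walks the hero toward a destination.
; When BP_Hero overlaps it, the player's view blends to this actor and the player controller unpossesses its pawn.
; The hero then gets its default controller spawned, and AIMoveTo sends it to a random navigable point close to the Destination component.
; The file contains no logic to restore player control afterward.
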(event `self.ReceiveActorBeginOverlap`
  (params (OtherActor :type "Actor Object Reference"))
  (bind _asbp_hero (cast `/Game/SEFAR/Core/BluePrints/BP_Hero` OtherActor))
  (bind _output_get (set `self.Controller` (`GameplayStatics.GetPlayerController` 0)))
  (`PlayerController.SetViewTargetWithBlend` (`self.Controller`) self 1.0 "VTBlend_Linear" 0.0 false)
  (`Controller.UnPossess` _output_get)
  (`Pawn.SpawnDefaultController` _asbp_hero)
  (`|AIMoveTo` _asbp_hero (`NavigationSystemV1.K2_GetRandomLocationInNavigableRadius` (`SceneComponent.K2_GetComponentLocation` (`self.Destination`)) 50.0 null null) null))

(fn `UserConstructionScript`)