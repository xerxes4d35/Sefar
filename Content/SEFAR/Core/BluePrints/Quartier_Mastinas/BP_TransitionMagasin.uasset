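; BP_TransitionMagasin is a trigger actor that plays a scripted walk-in transition from the level to the Magasin_Adam shop level.
; On the hero's first overlap, it blends the player's view to itself, unpossesses the hero and gives it a default controller.
; AI MoveTo walks the hero near the Destination component, then opens the shop level on success.
; Each hero overlap also applies the GameInstance subtitle setting.
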(event `self.ReceiveActorBeginOverlap`
  (params (OtherActor :type "Actor Object Reference"))
  (bind _bp_hero (`self.BP Hero`))
  (bind _asbp_hero (cast `/Game/SEFAR/Core/BluePrints/BP_Hero` OtherActor))
  (set `self.BP Hero` _asbp_hero)
  (bind _asbp_game_instance (cast `/Game/SEFAR/Core/BluePrints/BP_GameInstance` (`GameplayStatics.GetGameInstance`)))
  (if (`/Game/SEFAR/Core/BluePrints/BP_GameInstance.Subtitles` _asbp_game_instance)
    (`GameplayStatics.SetSubtitlesEnabled` true)
    (else
      (`GameplayStatics.SetSubtitlesEnabled` false)))
  (if (not (`self.GetOverlapped`))
    (bind _output_get (set `self.Controller` (`GameplayStatics.GetPlayerController` 0)))
    (`PlayerController.SetViewTargetWithBlend` (`self.Controller`) self 1.0 "VTBlend_Linear" 0.0 false)
    (set `self.GetOverlapped` true)
    (`Controller.UnPossess` _output_get)
    (`Pawn.SpawnDefaultController` _bp_hero)
    (`|AIMoveTo` _bp_hero (`NavigationSystemV1.K2_GetRandomLocationInNavigableRadius` (`SceneComponent.K2_GetComponentLocation` (`self.Destination`)) 50.0 null null) null
      (:`OnSuccess`
        (`GameplayStatics.OpenLevel` "Magasin_Adam")))))

(fn `UserConstructionScript`)