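; BP_DialoguePNJ_Femme is a proximity trigger that plays a female NPC's voice dialogue when the player enters its box.
; The first overlap spawns the dialogue sound at the actor's location and stores the audio component behind a done flag, so it never restarts.
; Leaving the box mutes that component and turns subtitles off, while re-entering restores the volume and turns subtitles back on.
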(event `self.Box.OnComponentBeginOverlap`
  (params (OverlappedComponent :type "PrimitiveComponent Object Reference") (OtherActor :type "Actor Object Reference") (OtherComp :type "PrimitiveComponent Object Reference") (OtherBodyIndex :type Integer) (bFromSweep :type Boolean) (SweepResult :type "HitResult Structure (by ref)"))
  (if (== OtherActor (`GameplayStatics.GetPlayerCharacter` 0))
    (if (`self.IsDialogueDOne`)
      (`AudioComponent.SetVolumeMultiplier` (`self.Dialogue Femme`) 1.0)
      (`GameplayStatics.SetSubtitlesEnabled` true)
      (else
        (bind _returnvalue (`GameplayStatics.SpawnSoundAtLocation` "/Game/SEFAR/Sound/Dialogue/Quartier_Mastinas/Dialogue_Femme.Dialogue_Femme" (`self.K2_GetActorLocation` self) (struct) 1.0 1.0 0.0 null null))
        (set `self.Dialogue Femme` _returnvalue)
        (set `self.IsDialogueDOne` true)))))

(event `self.Box.OnComponentEndOverlap`
  (params (OverlappedComponent :type "PrimitiveComponent Object Reference") (OtherActor :type "Actor Object Reference") (OtherComp :type "PrimitiveComponent Object Reference") (OtherBodyIndex :type Integer))
  (if (== OtherActor (`GameplayStatics.GetPlayerCharacter` 0))
    (`AudioComponent.SetVolumeMultiplier` (`self.Dialogue Femme`) 0.0)
    (`GameplayStatics.SetSubtitlesEnabled` false)))

(fn `UserConstructionScript`)