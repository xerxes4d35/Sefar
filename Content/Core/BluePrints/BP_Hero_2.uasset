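; Player hero Blueprint that handles world-axis movement, look rotation and a four-app phone menu (SMS, Astera, News, Options).
; BeginPlay creates the HUD and phone widgets and temporarily unlocks Astera, which navigation otherwise skips.
; NumMenu, FocusLevel and LevelOneCounter drive app switching, focus depth and SMS/News item highlighting, while an open menu blocks movement.
; Vertical axis input is latched in Operator and applied on stick release, giving one step per press.
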(event `self.ReceiveBeginPlay`
  ;[1 1 1] Begin events
  (bind _returnvalue (`|CreateWidget` "/Game/UI/WBP_IngameHUD.WBP_IngameHUD_C"))
  (bind _output_get (set `self.HUD` _returnvalue))
  (`UserWidget.AddToViewport` _output_get 0)
  (bind _returnvalue_2 (`|CreateWidget` "/Game/UI/WBP_PhoneSMS.WBP_PhoneSMS_C"))
  (bind _output_get_2 (set `self.WidgetSMS` _returnvalue_2))
  (bind _returnvalue_3 (`|CreateWidget` "/Game/UI/WBP_PhoneAstera.WBP_PhoneAstera_C"))
  (bind _output_get_3 (set `self.WidgetAstera` _returnvalue_3))
  (bind _returnvalue_4 (`|CreateWidget` "/Game/UI/WBP_PhoneNews.WBP_PhoneNews_C"))
  (bind _output_get_4 (set `self.WidgetNews` _returnvalue_4))
  (bind _returnvalue_5 (`|CreateWidget` "/Game/UI/WBP_PhoneOptions.WBP_PhoneOptions_C"))
  (bind _output_get_5 (set `self.WidgetOptions` _returnvalue_5))
  (`Widget.SetVisibility` _output_get_2 "Collapsed")
  (`Widget.SetVisibility` _output_get_5 "Collapsed")
  (`Widget.SetVisibility` _output_get_3 "Collapsed")
  (`Widget.SetVisibility` _output_get_4 "Collapsed")
  (`UserWidget.AddToViewport` _output_get_2 0)
  (`UserWidget.AddToViewport` _output_get_3 0)
  (`UserWidget.AddToViewport` _output_get_4 0)
  (`UserWidget.AddToViewport` _output_get_5 0)
  ;[1 1 1] Temporaire
  (`self.UnlockAstera`))

(event `InputAxis|LookUp`
  (params (AxisValue :type "Float (single-precision)"))
  ;[1 1 1] Rotation
  (if (not (`self.MenuIsOpen`)) :!label _label
    (bind _returnvalue (`KismetMathLibrary.MakeVector` AxisValue (stale `InputAxis|LookRight` AxisValue)))
    (if (> (`KismetMathLibrary.VSize` _returnvalue) 0.01)
      (`Controller.SetControlRotation` (`GameplayStatics.GetPlayerController` 0) (`KismetMathLibrary.Conv_VectorToRotator` _returnvalue)))))

(event `InputAxis|MoveUP`
  (params (AxisValue :type "Float (single-precision)"))
  ;[1 1 1] Movement
  (if (not (`self.MenuIsOpen`))
    (`self.AddMovementInput` (1.0 0.0 0.0) AxisValue)))

(event `InputAction|MenuCancel`
  (params (Key :type "Key Structure"))
  ;[1 1 1] Menu cancel (focus level -1)
  (:`Released`
    (if (`self.MenuIsOpen`) :!label _label_2
      (switch `int` (`self.FocusLevel`)
        (:`1`
          (if (== (`self.NumMenu`) 0)
            (`|ExecutionSequence`
              (:`then_0`
                (set `self.FocusLevel` 0 :!label _label_3)
                (set `self.LevelOneCounter` 0)
                (switch `int` (`self.NumMenu`) :!label _label_4 ; Switch on apps
                  (:`0`
                    (`self.ResetSMSBorder`))
                  (:`1`
                    (bind _aswbp_phone_astera (cast `/Game/UI/WBP_PhoneAstera` (`self.WidgetAstera`)))
                    (`Image.SetColorAndOpacity` (`/Game/UI/WBP_PhoneAstera.Image_Border` _aswbp_phone_astera) (struct :`R` 0.708376 :`G` 0.401978 :`B` 0.068478 :`A` 1.0)))
                  (:`2`
                    (bind _aswbp_phone_news (cast `/Game/UI/WBP_PhoneNews` (`self.WidgetNews`)))
                    (`Image.SetColorAndOpacity` (`/Game/UI/WBP_PhoneNews.Image_Border` _aswbp_phone_news) (struct :`R` 0.708376 :`G` 0.401978 :`B` 0.068478 :`A` 1.0)))
                  (:`3`
                    (bind _aswbp_phone_options (cast `/Game/UI/WBP_PhoneOptions` (`self.WidgetOptions`)))
                    (`Image.SetColorAndOpacity` (`/Game/UI/WBP_PhoneOptions.Image_Border` _aswbp_phone_options) (struct :`R` 0.708376 :`G` 0.401978 :`B` 0.068478 :`A` 1.0)))))
              (:`then_1`
                ;[1 1 1] Focus Level 1 Navigation (Vertical)
                ;;[1 1 1] SMS Part
                (bind _aswbp_phone_sms (cast `/Game/UI/WBP_PhoneSMS` (`self.WidgetSMS`) :!label _label_5))
                (switch `int` (`self.LevelOneCounter`)
                  (:`0`
                    (if (== (`self.FocusLevel`) 0)
                      (bind _border_cornelius (`/Game/UI/WBP_PhoneSMS.Border_Cornelius` _aswbp_phone_sms))
                      (`Border.SetBrushColor` _border_cornelius (struct :`R` 0.026241 :`G` 0.026241 :`B` 0.026241 :`A` 0.75))
                      (bind _border_fitness (`/Game/UI/WBP_PhoneSMS.Border_Fitness` _aswbp_phone_sms))
                      (`Border.SetBrushColor` _border_fitness (struct :`R` 0.026241 :`G` 0.026241 :`B` 0.026241 :`A` 0.75))
                      (bind _border_sirine (`/Game/UI/WBP_PhoneSMS.Border_Sirine` _aswbp_phone_sms))
                      (`Border.SetBrushColor` _border_sirine (struct :`R` 0.026241 :`G` 0.026241 :`B` 0.026241 :`A` 0.75))
                      (bind _border_unknown_1 (`/Game/UI/WBP_PhoneSMS.Border_Unknown_1` _aswbp_phone_sms))
                      (`Border.SetBrushColor` _border_unknown_1 (struct :`R` 0.026241 :`G` 0.026241 :`B` 0.026241 :`A` 0.75))
                      (bind _border_unknown_2 (`/Game/UI/WBP_PhoneSMS.Border_Unknown_2` _aswbp_phone_sms))
                      (`Border.SetBrushColor` _border_unknown_2 (struct :`R` 0.026241 :`G` 0.026241 :`B` 0.026241 :`A` 0.75))
                      (set `self.Operator` 0)
                      (`self.ResetSMSBorder`)
                      (else
                        (`Border.SetBrushColor` _border_cornelius (struct :`R` 0.109462 :`G` 0.109462 :`B` 0.109462 :`A` 0.75))
                        (`|ExecutionSequence`
                          (:`then_0`
                            (`Border.SetBrushColor` _border_fitness (struct :`R` 0.026241 :`G` 0.026241 :`B` 0.026241 :`A` 0.75) :!label _label_6))
                          (:`then_1`
                            (`Border.SetBrushColor` _border_sirine (struct :`R` 0.026241 :`G` 0.026241 :`B` 0.026241 :`A` 0.75) :!label _label_7))
                          (:`then_2`
                            (`Border.SetBrushColor` _border_unknown_1 (struct :`R` 0.026241 :`G` 0.026241 :`B` 0.026241 :`A` 0.75) :!label _label_8))
                          (:`then_3`
                            (`Border.SetBrushColor` _border_unknown_2 (struct :`R` 0.026241 :`G` 0.026241 :`B` 0.026241 :`A` 0.75) :!label _label_9)))
                        (set `self.Operator` 0 :!label _label_10)
                        (`self.ResetSMSBorder`)
                        (`self.ColorSMSBorder` (`self.LevelOneCounter`)))))
                  (:`1`
                    (`Border.SetBrushColor` _border_fitness (struct :`R` 0.109462 :`G` 0.109462 :`B` 0.109462 :`A` 0.75))
                    (`|ExecutionSequence`
                      (:`then_0`
                        (`Border.SetBrushColor` _border_cornelius (struct :`R` 0.026241 :`G` 0.026241 :`B` 0.026241 :`A` 0.75) :!label _label_11)
                        (goto _label_10))
                      (:`then_1`
                        (goto _label_7))
                      (:`then_2`
                        (goto _label_8))
                      (:`then_3`
                        (goto _label_9))))
                  (:`2`
                    (`Border.SetBrushColor` _border_sirine (struct :`R` 0.109462 :`G` 0.109462 :`B` 0.109462 :`A` 0.75))
                    (`|ExecutionSequence`
                      (:`then_0`
                        (goto _label_11))
                      (:`then_1`
                        (goto _label_6))
                      (:`then_2`
                        (goto _label_8))
                      (:`then_3`
                        (goto _label_9))))
                  (:`3`
                    (`Border.SetBrushColor` _border_unknown_1 (struct :`R` 0.109462 :`G` 0.109462 :`B` 0.109462 :`A` 0.75))
                    (`|ExecutionSequence`
                      (:`then_0`
                        (goto _label_11))
                      (:`then_1`
                        (goto _label_6))
                      (:`then_2`
                        (goto _label_7))
                      (:`then_3`
                        (goto _label_9))))
                  (:`4`
                    (`Border.SetBrushColor` _border_unknown_2 (struct :`R` 0.109462 :`G` 0.109462 :`B` 0.109462 :`A` 0.75))
                    (`|ExecutionSequence`
                      (:`then_0`
                        (goto _label_11))
                      (:`then_1`
                        (goto _label_6))
                      (:`then_2`
                        (goto _label_7))
                      (:`then_3`
                        (goto _label_8)))))))
            (elif (== (`self.NumMenu`) 2)
              (`|ExecutionSequence`
                (:`then_0`
                  (goto _label_3))
                (:`then_1`
                  ;;[1 1 1] News Part
                  (bind _aswbp_phone_news_2 (cast `/Game/UI/WBP_PhoneNews` (`self.WidgetNews`) :!label _label_12))
                  (switch `int` (`self.LevelOneCounter`)
                    (:`0`
                      (if (== (`self.FocusLevel`) 0)
                        (bind _border_article_1 (`/Game/UI/WBP_PhoneNews.Border_Article_1` _aswbp_phone_news_2))
                        (`Border.SetBrushColor` _border_article_1 (struct :`R` 0.026241 :`G` 0.026241 :`B` 0.026241 :`A` 0.75))
                        (bind _border_article_2 (`/Game/UI/WBP_PhoneNews.Border_Article_2` _aswbp_phone_news_2))
                        (`Border.SetBrushColor` _border_article_2 (struct :`R` 0.026241 :`G` 0.026241 :`B` 0.026241 :`A` 0.75))
                        (bind _border_article_3 (`/Game/UI/WBP_PhoneNews.Border_Article_3` _aswbp_phone_news_2))
                        (`Border.SetBrushColor` _border_article_3 (struct :`R` 0.026241 :`G` 0.026241 :`B` 0.026241 :`A` 0.75))
                        (bind _border_article_4 (`/Game/UI/WBP_PhoneNews.Border_Article_4` _aswbp_phone_news_2))
                        (`Border.SetBrushColor` _border_article_4 (struct :`R` 0.026241 :`G` 0.026241 :`B` 0.026241 :`A` 0.75))
                        (set `self.Operator` 0)
                        (`self.ResetNewsBorder`)
                        (else
                          (`Border.SetBrushColor` _border_article_1 (struct :`R` 0.109462 :`G` 0.109462 :`B` 0.109462 :`A` 0.75))
                          (`|ExecutionSequence`
                            (:`then_0`
                              (`Border.SetBrushColor` _border_article_2 (struct :`R` 0.026241 :`G` 0.026241 :`B` 0.026241 :`A` 0.75) :!label _label_13))
                            (:`then_1`
                              (`Border.SetBrushColor` _border_article_3 (struct :`R` 0.026241 :`G` 0.026241 :`B` 0.026241 :`A` 0.75) :!label _label_14))
                            (:`then_2`
                              (`Border.SetBrushColor` _border_article_4 (struct :`R` 0.026241 :`G` 0.026241 :`B` 0.026241 :`A` 0.75) :!label _label_15)))
                          (set `self.Operator` 0 :!label _label_16)
                          (`self.ResetNewsBorder`)
                          (`self.ColorNewsBorder` (`self.LevelOneCounter`)))))
                    (:`1`
                      (`Border.SetBrushColor` _border_article_2 (struct :`R` 0.109462 :`G` 0.109462 :`B` 0.109462 :`A` 0.75))
                      (`|ExecutionSequence`
                        (:`then_0`
                          (`Border.SetBrushColor` _border_article_1 (struct :`R` 0.026241 :`G` 0.026241 :`B` 0.026241 :`A` 0.75) :!label _label_17)
                          (goto _label_16))
                        (:`then_1`
                          (goto _label_14))
                        (:`then_2`
                          (goto _label_15))))
                    (:`2`
                      (`Border.SetBrushColor` _border_article_3 (struct :`R` 0.109462 :`G` 0.109462 :`B` 0.109462 :`A` 0.75))
                      (`|ExecutionSequence`
                        (:`then_0`
                          (goto _label_17))
                        (:`then_1`
                          (goto _label_13))
                        (:`then_2`
                          (goto _label_15))))
                    (:`3`
                      (`Border.SetBrushColor` _border_article_4 (struct :`R` 0.109462 :`G` 0.109462 :`B` 0.109462 :`A` 0.75))
                      (`|ExecutionSequence`
                        (:`then_0`
                          (goto _label_17))
                        (:`then_1`
                          (goto _label_13))
                        (:`then_2`
                          (goto _label_14)))))))
              (else
                (goto _label_3)))))
        (:`2`
          (set `self.FocusLevel` 1))))))

(event `InputAxis|LookRight`
  (params (AxisValue :type "Float (single-precision)"))
  ;[1 1 1] Rotation
  (goto _label))

(event `InputAxis|MoveRight`
  (params (AxisValue :type "Float (single-precision)"))
  ;[1 1 1] Movement
  (if (not (`self.MenuIsOpen`))
    (`self.AddMovementInput` (0.0 1.0 0.0) AxisValue)))

(event `InputAction|MenuOpenClose`
  (params (Key :type "Key Structure"))
  ;[1 1 1] Open & Close the HUD
  (:`Released`
    (if (`self.MenuIsOpen`)
      (`Widget.SetVisibility` (`self.WidgetSMS`) "Collapsed")
      (`Widget.SetVisibility` (`self.WidgetAstera`) "Collapsed")
      (`Widget.SetVisibility` (`self.WidgetNews`) "Collapsed")
      (`Widget.SetVisibility` (`self.WidgetOptions`) "Collapsed")
      (`Widget.SetVisibility` (`self.HUD`) "Visible")
      (set `self.MenuIsOpen` false)
      (set `self.Operator` 0)
      (set `self.FocusLevel` 0)
      (set `self.LevelOneCounter` 0)
      (`|ExecutionSequence`
        (:`then_0`
          (goto _label_4))
        (:`then_1`
          (set `self.NumMenu` 0)))
      (else
        (`Widget.SetVisibility` (`self.HUD`) "Collapsed") ; Open
        (bind _output_get (set `self.CurrentUI` (`self.WidgetSMS`)))
        (`Widget.SetVisibility` _output_get "Visible")
        (set `self.MenuIsOpen` true)))))

(event `InputAxis|MenuMoveUp`
  (params (AxisValue :type "Float (single-precision)"))
  (bind _levelonecounter (`self.LevelOneCounter`))
  (bind _levelonecounter_2 (`self.LevelOneCounter`))
  (bind _widgetsms (`self.WidgetSMS`))
  (bind _widgetastera (`self.WidgetAstera`))
  (bind _widgetnews (`self.WidgetNews`))
  (bind _widgetoptions (`self.WidgetOptions`))
  (bind _levelonecounter_3 (`self.LevelOneCounter`))
  (bind _levelonecounter_4 (`self.LevelOneCounter`))
  (if (`self.MenuIsOpen`)
    (if (> AxisValue 0.2)
      (set `self.Operator` 1)
      (elif (< AxisValue -0.2)
        (set `self.Operator` -1)
        (else
          (switch `int` (`self.FocusLevel`) ; Focus level cases
            (:`0`
              ;[1 1 1] Menu Icons Navigation (Vertical)
              (switch `int` (`self.Operator`) ; Key released
                (:`-1`
                  (bind _output_get (set `self.NumMenu` (+ (`self.NumMenu`) 1)))
                  (if (== _output_get 1)
                    (if (not (`self.AsteraUnlocked`))
                      (set `self.NumMenu` 2))
                    (elif (> (`self.NumMenu`) 3)
                      (set `self.NumMenu` 0))))
                (:`1`
                  (bind _output_get_2 (set `self.NumMenu` (- (`self.NumMenu`) 1)))
                  (if (== _output_get_2 1)
                    (if (not (`self.AsteraUnlocked`))
                      (set `self.NumMenu` 0))
                    (elif (< (`self.NumMenu`) 0)
                      (set `self.NumMenu` 3)))))
              (switch `int` (`self.NumMenu`)
                (:`0`
                  (`Widget.SetVisibility` _widgetsms "Visible")
                  (`|ExecutionSequence`
                    (:`then_0`
                      (`Widget.SetVisibility` _widgetastera "Collapsed" :!label _label_18))
                    (:`then_1`
                      (`Widget.SetVisibility` _widgetnews "Collapsed" :!label _label_19))
                    (:`then_2`
                      (`Widget.SetVisibility` _widgetoptions "Collapsed" :!label _label_20))))
                (:`1`
                  (`Widget.SetVisibility` _widgetastera "Visible")
                  (`|ExecutionSequence`
                    (:`then_0`
                      (`Widget.SetVisibility` _widgetsms "Collapsed" :!label _label_21))
                    (:`then_1`
                      (goto _label_19))
                    (:`then_2`
                      (goto _label_20))))
                (:`2`
                  (`Widget.SetVisibility` _widgetnews "Visible")
                  (`|ExecutionSequence`
                    (:`then_0`
                      (goto _label_21))
                    (:`then_1`
                      (goto _label_18))
                    (:`then_2`
                      (goto _label_20))))
                (:`3`
                  (`Widget.SetVisibility` _widgetoptions "Visible")
                  (`|ExecutionSequence`
                    (:`then_0`
                      (goto _label_21))
                    (:`then_1`
                      (goto _label_18))
                    (:`then_2`
                      (goto _label_19)))))
              (set `self.Operator` 0))
            (:`1`
              ;[1 1 1] Focus Level 1 Navigation (Vertical)
              (switch `int` (`self.NumMenu`) ; Application cases
                (:`0`
                  ;;[1 1 1] SMS Part
                  (switch `int` (`self.Operator`) ; Key released
                    (:`-1`
                      (set `self.LevelOneCounter` (+ _levelonecounter 1))
                      (if (> _levelonecounter 4)
                        (set `self.LevelOneCounter` 0)
                        (goto _label_5)
                        (else
                          (goto _label_5))))
                    (:`1`
                      (set `self.LevelOneCounter` (- _levelonecounter_2 1))
                      (if (< _levelonecounter_2 0)
                        (set `self.LevelOneCounter` 4)
                        (goto _label_5)
                        (else
                          (goto _label_5))))))
                (:`1`
                  ;;[1 1 1] Astera Part
                  (switch `int` (`self.Operator`) ; Key released
                    (:`-1`
                      _)
                    (:`1`
                      _))
                  (set `self.Operator` 0))
                (:`2`
                  ;;[1 1 1] News Part
                  (switch `int` (`self.Operator`) ; Key released
                    (:`-1`
                      (set `self.LevelOneCounter` (+ _levelonecounter_3 1))
                      (if (> _levelonecounter_3 3)
                        (set `self.LevelOneCounter` 0)
                        (goto _label_12)
                        (else
                          (goto _label_12))))
                    (:`1`
                      (set `self.LevelOneCounter` (- _levelonecounter_4 1))
                      (if (< _levelonecounter_4 0)
                        (set `self.LevelOneCounter` 3)
                        (goto _label_12)
                        (else
                          (goto _label_12))))))
                (:`3`
                  ;;[1 1 1] Options Part
                  (switch `int` (`self.Operator`) ; Key released
                    (:`-1`
                      _)
                    (:`1`
                      _))
                  (set `self.Operator` 0))))))))))

(event `InputAxis|MenuMoveRight`
  (params (AxisValue :type "Float (single-precision)"))
  (if (and (and (> (stale `InputAxis|MenuMoveUp` AxisValue) -0.2) (< (stale `InputAxis|MenuMoveUp` AxisValue) 0.2)) (`self.MenuIsOpen`))
    (if (> AxisValue 0.2)
      (set `self.OperatorHorizontal` 1)
      (elif (< AxisValue -0.2)
        (set `self.OperatorHorizontal` -1)
        (else
          (switch `int` (`self.FocusLevel`) ; Focus level cases
            (:`0`
              ;[1 1 1] Validate Focus Level 0
              (switch `int` (`self.OperatorHorizontal`) ; Key released
                (:`-1`
                  (set `self.OperatorHorizontal` 0))
                (:`1`
                  (set `self.FocusLevel` 1 :!label _label_22)
                  (set `self.LevelOneCounter` 0)
                  (set `self.OperatorHorizontal` 0)
                  (switch `int` (`self.NumMenu`) ; Switch on apps
                    (:`0`
                      (bind _aswbp_phone_sms (cast `/Game/UI/WBP_PhoneSMS` (`self.WidgetSMS`)))
                      (`Image.SetColorAndOpacity` (`/Game/UI/WBP_PhoneSMS.Image_Cadre` _aswbp_phone_sms) (struct :`G` 0.646464 :`B` 0.679543 :`A` 1.0))
                      (`Border.SetBrushColor` (`/Game/UI/WBP_PhoneSMS.Border_Cornelius` _aswbp_phone_sms) (struct :`R` 0.109462 :`G` 0.109462 :`B` 0.109462 :`A` 0.75)))
                    (:`1`
                      (bind _aswbp_phone_astera (cast `/Game/UI/WBP_PhoneAstera` (`self.WidgetAstera`)))
                      (`Image.SetColorAndOpacity` (`/Game/UI/WBP_PhoneAstera.Image_Border` _aswbp_phone_astera) (struct :`G` 0.679543 :`B` 0.603828 :`A` 1.0)))
                    (:`2`
                      (bind _aswbp_phone_news (cast `/Game/UI/WBP_PhoneNews` (`self.WidgetNews`)))
                      (`Image.SetColorAndOpacity` (`/Game/UI/WBP_PhoneNews.Image_Cadre` _aswbp_phone_news) (struct :`G` 0.646464 :`B` 0.679543 :`A` 1.0))
                      (`Border.SetBrushColor` (`/Game/UI/WBP_PhoneNews.Border_Article_1` _aswbp_phone_news) (struct :`R` 0.109462 :`G` 0.109462 :`B` 0.109462 :`A` 0.75)))
                    (:`3`
                      (bind _aswbp_phone_options (cast `/Game/UI/WBP_PhoneOptions` (`self.WidgetOptions`)))
                      (`Image.SetColorAndOpacity` (`/Game/UI/WBP_PhoneOptions.Image_Border` _aswbp_phone_options) (struct :`G` 0.679543 :`B` 0.603828 :`A` 1.0)))))))
            (:`1`
              ;[1 1 1] Validate Focus Level 1
              (switch `int` (`self.OperatorHorizontal`) ; Key released
                (:`-1`
                  (set `self.OperatorHorizontal` 0)
                  (goto _label_2))
                (:`1`
                  (set `self.FocusLevel` 2 :!label _label_23)
                  (set `self.OperatorHorizontal` 0))))))))))

(event `InputAction|MenuValidate`
  (params (Key :type "Key Structure"))
  (:`Released`
    (if (`self.MenuIsOpen`)
      (switch `int` (`self.FocusLevel`)
        (:`0`
          (goto _label_22))
        (:`1`
          (goto _label_23))))))

(fn `ColorNewsBorder`
  (params (NumBorder :type Integer))
  (bind _aswbp_phone_news (cast `/Game/UI/WBP_PhoneNews` (`self.WidgetNews`)))
  (switch `int` NumBorder
    (:`Default`
      (`Image.SetColorAndOpacity` (`/Game/UI/WBP_PhoneNews.Image_Cadre` _aswbp_phone_news) (struct :`G` 1.0 :`B` 0.990156 :`A` 1.0) :!label _label))
    (:`0`
      (goto _label))
    (:`1`
      (`Image.SetColorAndOpacity` (`/Game/UI/WBP_PhoneNews.Image_Cadre_1` _aswbp_phone_news) (struct :`G` 1.0 :`B` 0.990156 :`A` 1.0)))
    (:`2`
      (`Image.SetColorAndOpacity` (`/Game/UI/WBP_PhoneNews.Image_Cadre_2` _aswbp_phone_news) (struct :`G` 1.0 :`B` 0.990156 :`A` 1.0)))
    (:`3`
      (`Image.SetColorAndOpacity` (`/Game/UI/WBP_PhoneNews.Image_Cadre_3` _aswbp_phone_news) (struct :`G` 1.0 :`B` 0.990156 :`A` 1.0)))))

(fn `ColorSMSBorder`
  (params (NumBorder :type Integer))
  (bind _aswbp_phone_sms (cast `/Game/UI/WBP_PhoneSMS` (`self.WidgetSMS`)))
  (switch `int` NumBorder
    (:`Default`
      (`Image.SetColorAndOpacity` (`/Game/UI/WBP_PhoneSMS.Image_Cadre` _aswbp_phone_sms) (struct :`G` 1.0 :`B` 0.990156 :`A` 1.0) :!label _label))
    (:`0`
      (goto _label))
    (:`1`
      (`Image.SetColorAndOpacity` (`/Game/UI/WBP_PhoneSMS.Image_Cadre_1` _aswbp_phone_sms) (struct :`G` 1.0 :`B` 0.990156 :`A` 1.0)))
    (:`2`
      (`Image.SetColorAndOpacity` (`/Game/UI/WBP_PhoneSMS.Image_Cadre_2` _aswbp_phone_sms) (struct :`G` 1.0 :`B` 0.990156 :`A` 1.0)))
    (:`3`
      (`Image.SetColorAndOpacity` (`/Game/UI/WBP_PhoneSMS.Image_Cadre_3` _aswbp_phone_sms) (struct :`G` 1.0 :`B` 0.990156 :`A` 1.0)))
    (:`4`
      (`Image.SetColorAndOpacity` (`/Game/UI/WBP_PhoneSMS.Image_Cadre_4` _aswbp_phone_sms) (struct :`G` 1.0 :`B` 0.990156 :`A` 1.0)))))

(fn `ResetNewsBorder`
  (bind _aswbp_phone_news (cast `/Game/UI/WBP_PhoneNews` (`self.WidgetNews`)))
  (`Image.SetColorAndOpacity` (`/Game/UI/WBP_PhoneNews.Image_Cadre` _aswbp_phone_news) (struct :`R` 1.0 :`G` 1.0 :`B` 1.0 :`A` 1.0))
  (`Image.SetColorAndOpacity` (`/Game/UI/WBP_PhoneNews.Image_Cadre_1` _aswbp_phone_news) (struct :`R` 1.0 :`G` 1.0 :`B` 1.0 :`A` 1.0))
  (`Image.SetColorAndOpacity` (`/Game/UI/WBP_PhoneNews.Image_Cadre_2` _aswbp_phone_news) (struct :`R` 1.0 :`G` 1.0 :`B` 1.0 :`A` 1.0))
  (`Image.SetColorAndOpacity` (`/Game/UI/WBP_PhoneNews.Image_Cadre_3` _aswbp_phone_news) (struct :`R` 1.0 :`G` 1.0 :`B` 1.0 :`A` 1.0)))

(fn `ResetSMSBorder`
  (bind _aswbp_phone_sms (cast `/Game/UI/WBP_PhoneSMS` (`self.WidgetSMS`)))
  (`Image.SetColorAndOpacity` (`/Game/UI/WBP_PhoneSMS.Image_Cadre_1` _aswbp_phone_sms) (struct :`R` 1.0 :`G` 1.0 :`B` 1.0 :`A` 1.0))
  (`Image.SetColorAndOpacity` (`/Game/UI/WBP_PhoneSMS.Image_Cadre` _aswbp_phone_sms) (struct :`R` 1.0 :`G` 1.0 :`B` 1.0 :`A` 1.0))
  (`Image.SetColorAndOpacity` (`/Game/UI/WBP_PhoneSMS.Image_Cadre_2` _aswbp_phone_sms) (struct :`R` 1.0 :`G` 1.0 :`B` 1.0 :`A` 1.0))
  (`Image.SetColorAndOpacity` (`/Game/UI/WBP_PhoneSMS.Image_Cadre_3` _aswbp_phone_sms) (struct :`R` 1.0 :`G` 1.0 :`B` 1.0 :`A` 1.0))
  (`Image.SetColorAndOpacity` (`/Game/UI/WBP_PhoneSMS.Image_Cadre_4` _aswbp_phone_sms) (struct :`R` 1.0 :`G` 1.0 :`B` 1.0 :`A` 1.0)))

(fn `UnlockAstera`
  ;[1 1 1] Unlock Astera
  (set `self.AsteraUnlocked` true)
  (bind _aswbp_phone_sms (cast `/Game/UI/WBP_PhoneSMS` (`self.WidgetSMS`)))
  (`Widget.SetVisibility` (`/Game/UI/WBP_PhoneSMS.Icon_Astera` _aswbp_phone_sms) "Visible")
  (`Widget.SetVisibility` (`/Game/UI/WBP_PhoneSMS.Round_Astera` _aswbp_phone_sms) "Visible")
  (bind _aswbp_phone_news (cast `/Game/UI/WBP_PhoneNews` (`self.WidgetNews`)))
  (`Widget.SetVisibility` (`/Game/UI/WBP_PhoneNews.Icon_Astera` _aswbp_phone_news) "Visible")
  (`Widget.SetVisibility` (`/Game/UI/WBP_PhoneNews.Round_Astera` _aswbp_phone_news) "Visible")
  (bind _aswbp_phone_options (cast `/Game/UI/WBP_PhoneOptions` (`self.WidgetOptions`)))
  (`Widget.SetVisibility` (`/Game/UI/WBP_PhoneOptions.Icon_Astera` _aswbp_phone_options) "Visible")
  (`Widget.SetVisibility` (`/Game/UI/WBP_PhoneOptions.Round_Astera` _aswbp_phone_options) "Visible"))

(fn `UserConstructionScript`
  (`parent.UserConstructionScript`))